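; BP_ScorePoint is a star pickup that awards score when a BP_ThirdPersonCharacter touches it.
; The star model spins by a fixed step each tick, independent of delta time.
; On box overlap it calls AddScore directly on the game UI widget held by GS_Parkour, spawns a NiagaraSystem actor at its transform, then destroys itself.
; A node deactivating Niagara1 is left unconnected.
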(event OnComponentBeginOverlap(Box)
  (params (OverlappedComponent :type Primitive%20Component%20Object%20Reference) (OtherActor :type Actor%20Object%20Reference) (OtherComp :type Primitive%20Component%20Object%20Reference) (OtherBodyIndex :type Integer) (bFromSweep :type Boolean) (SweepResult :type Hit%20Result%20Structure%20%28by%20ref%29))
  (Utilities|Casting|CastToBP_ThirdPersonCharacter OtherActor)
  (Default|AddScore (Variables|/Game/Nate/GS_Parkour.GS_Parkour_C|GetWB_GameUI (.AsGS%20Parkour (Utilities|Casting|CastToGS_Parkour (Game|GetGameState)))))
  (Game|SpawnActorfromClass (Variables|Default|GetNiagaraSystem) (Transformation|GetActorTransform self) "Undefined" 0 0)
  (Actor|DestroyActor))

(event EventBeginPlay)

(event EventTick
  (params (DeltaSeconds :type Float%20%28single-precision%29))
  (Transformation|AddLocalRotation (Variables|Default|GetStarModel) "0,1.000000, 0" false false))

(fn ConstructionScript)